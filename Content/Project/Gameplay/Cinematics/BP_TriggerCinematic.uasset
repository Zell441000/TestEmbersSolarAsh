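; Trigger volume actor that plays a level sequence cinematic when the player enters its box.
; The first overlap hides the player for the cinematic, plays the sequence, then after a short delay moves and rotates the player to the TPEnd transform.
; When the sequence finishes, CineEnd destroys the Skeletal actor and unhides the player.
; DoOnce precedes the BP_Player cast, so a non-player overlap also consumes the trigger.
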(event OnComponentBeginOverlap(Box)
  (params (OverlappedComponent :type Primitive%20Component%20Object%20Reference) (OtherActor :type Actor%20Object%20Reference) (OtherComp :type Primitive%20Component%20Object%20Reference) (OtherBodyIndex :type Integer) (bFromSweep :type Boolean) (SweepResult :type Hit%20Result%20Structure%20%28by%20ref%29))
  (bind _player (CallFunction|GetMyPlayer))
  (bind _cinematic (Variables|Default|GetCinematic))
  (bind _tpend (Variables|Default|GetTPEnd))
  (bind _returnvalue (Transformation|GetActorTransform _tpend))
  (bind _sequenceplayer (Variables|/Script/LevelSequence.LevelSequenceActor|GetSequencePlayer _cinematic))
  (Utilities|FlowControl|DoOnce false
    (:Completed
      (Utilities|Casting|CastToBP_Player OtherActor)
      (Default|HideDuringCine (CallFunction|GetMyPlayer) true)
      (Sequencer|Player|Play _sequenceplayer :!class /Script/MovieScene.MovieSceneSequencePlayer)
      (EventDispatchers|BindEventtoOnFinished _sequenceplayer (delegate Custom|CineEnd))
      (Utilities|FlowControl|Delay 2.0)
      (Transformation|SetActorLocation _player (.location _returnvalue) false false)
      (Transformation|SetActorRotation _player (.rotation _returnvalue)))))

(event Custom|CineEnd
  (Actor|DestroyActor (Variables|Default|GetSkeletal))
  (Default|HideDuringCine (CallFunction|GetMyPlayer) false))

(event EventBeginPlay)

(event Collision|EventActorBeginOverlap
  (params (OtherActor :type Actor%20Object%20Reference)))

(event EventTick
  (params (DeltaSeconds :type Float%20%28single-precision%29)))

(fn ConstructionScript)